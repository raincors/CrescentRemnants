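; Protagonist Blueprint with an early ledge-climb detection mechanic triggered by pressing Space Bar.
; DetermineClimbLocation sphere-traces forward from above the actor origin and stores the impact point in ForwardTraceHit.
; On a hit, a second debug-drawn trace probes downward from above that point, but its result is unused.
; No climbing movement is implemented, and releasing Space only prints a message.
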(event EventBeginPlay)

(event Collision|EventActorBeginOverlap
  (params (OtherActor :type Actor%20Object%20Reference)))

(event EventTick
  (params (DeltaSeconds :type Float%20%28single-precision%29)))

(event Input|KeyboardEvents|SpaceBar
  (params (Key :type Key%20Structure :default "None"))
  (:Pressed
    (CallFunction|DetermineClimbLocation))
  (:Released
    (Development|PrintString "Spacebar Released")))

(fn ConstructionScript)

(fn DetermineClimbLocation
  (bind _returnvalue (Transformation|GetActorLocation))
  (bind _returnvalue_2 (+ _returnvalue "0.000000,0.000000,90.000000"))
  (bind (_outhit _returnvalue_3) (Collision|SphereTraceByChannel _returnvalue_2 (+ _returnvalue_2 (* (Math|Vector|GetForwardVector (Transformation|GetActorRotation)) "150.000000,150.000000,150.000000")) 5.0 "TraceTypeQuery1" false 0 "ForDuration"))
  (if _returnvalue_3
    (LocalVariables|SetForwardTraceHit (.ImpactPoint (Collision|BreakHitResult _outhit)))
    (Collision|SphereTraceByChannel (+ (.ImpactPoint (Collision|BreakHitResult _outhit)) "0.000000,0.000000,90.000000") (- (+ (.ImpactPoint (Collision|BreakHitResult _outhit)) "0.000000,0.000000,90.000000") "0.000000,0.000000,95.000000") 6.0 "TraceTypeQuery1" false 0 "ForDuration")))