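; Protagonist character Blueprint with hold-Shift running and ledge detection for climbing while airborne.
; While falling, each Tick runs DetermineClimbLocation, which sphere-traces forward for a wall, then downward from above the hit for a ledge top.
; A valid ledge sets the climb location and wall-facing rotation, then attaches and positions ClimbSpot on the hit component.
; Success calls ExecuteClimbing, which is an empty event here.
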(event Custom|ExecuteClimbing)

(event EventBeginPlay)

(event Collision|EventActorBeginOverlap
  (params (OtherActor :type Actor%20Object%20Reference)))

(event EventTick
  (params (DeltaSeconds :type Float%20%28single-precision%29))
  (if (AI|Components|NavMovement|IsFalling (Variables|Character|GetCharacterMovement))
    (bind _enableclimbing (CallFunction|DetermineClimbLocation))
    (if _enableclimbing
      (CallFunction|ExecuteClimbing))))

(event Input|KeyboardEvents|LeftShift
  (params (Key :type Key%20Structure :default "None"))
  (:Pressed
    (Variables|/Script/Engine.CharacterMovementComponent|SetMaxWalkSpeed (Variables|Character|GetCharacterMovement) (Variables|Default|GetRunSpeed)))
  (:Released
    (Variables|/Script/Engine.CharacterMovementComponent|SetMaxWalkSpeed (Variables|Character|GetCharacterMovement) (Variables|Default|GetWalkSpeed))))

(fn ConstructionScript)

(fn DetermineClimbLocation
  (bind _returnvalue (Transformation|GetActorLocation))
  (bind _returnvalue_2 (+ _returnvalue "0.000000,0.000000,90.000000"))
  (bind (_outhit _returnvalue_3) (Collision|SphereTraceByChannel _returnvalue_2 (+ _returnvalue_2 (* (Math|Vector|GetForwardVector (Transformation|GetActorRotation)) "150.000000,150.000000,150.000000")) 5.0 "TraceTypeQuery1" false 0 "None"))
  (if _returnvalue_3
    (LocalVariables|SetForwardTraceHit (.ImpactPoint (Collision|BreakHitResult _outhit)))
    (LocalVariables|SetClimbRotation (Math|Rotator|Delta(Rotator) (Math|Rotator|MakeRotfromX (.ImpactNormal (Collision|BreakHitResult _outhit))) "0.000000,180.000000,0.000000"))
    (bind _outhit_2 (Collision|SphereTraceByChannel (+ (.ImpactPoint (Collision|BreakHitResult _outhit)) "0.000000,0.000000,90.000000") (- (+ (.ImpactPoint (Collision|BreakHitResult _outhit)) "0.000000,0.000000,90.000000") "0.000000,0.000000,95.000000") 6.0 "TraceTypeQuery1" false 0 "None"))
    (if (.bInitialOverlap (Collision|BreakHitResult _outhit_2))
      (bind _output_get (LocalVariables|SetEnableClimb false))
      (return _output_get)
      (elif (.bBlockingHit (Collision|BreakHitResult _outhit_2))
        (LocalVariables|SetHitComp (.HitComponent (Collision|BreakHitResult _outhit_2)))
        (LocalVariables|SetClimbLocation (Math|Vector|MakeVector (.x (- (LocalVariables|GetForwardTraceHit) (* (Math|Vector|GetForwardVector (LocalVariables|GetClimbRotation)) "45.000000,45.000000,45.000000"))) (.y (- (LocalVariables|GetForwardTraceHit) (* (Math|Vector|GetForwardVector (LocalVariables|GetClimbRotation)) "45.000000,45.000000,45.000000"))) (.z (- (.ImpactPoint (Collision|BreakHitResult _outhit_2)) "0.000000,0.000000,110.000000"))))
        (LocalVariables|SetEnableClimb true)
        (Transformation|AttachComponentToComponent (Variables|Default|GetClimbSpot) (LocalVariables|GetHitComp) "None" "KeepRelative" "KeepRelative" "KeepWorld" true)
        (Transformation|SetWorldLocationAndRotation (Variables|Default|GetClimbSpot) (LocalVariables|GetClimbLocation) (LocalVariables|GetClimbRotation) false false)
        (return (LocalVariables|GetEnableClimb))))
    (else
      (return false))))