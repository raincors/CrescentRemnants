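; BP_Protagonist_HUD is the player pawn that gathers memory remnants and opens the pause menu.
; Overlapping a BP_Collectible destroys it and advances the remnant progress ratio.
; Full progress increments Memory, plays a flashback sound, shows a timed WBP_TextBubble pop-up, then resets the remnant count once the bubble is removed.
; Releasing Escape pauses the game and shows WBP_Pause with UI-only input and a mouse cursor.
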(event Custom|UnlockMemory
  (if (>= (Variables|Default|GetRemnantsProgress) 1.0)
    (bind _result (Math|Integer|IncrementInt (Variables|Default|GetMemory))
      (:%20%20
        (Variables|Default|SetMemory _result)
        (Audio|PlaySound2D "/Game/Blueprints/HUD/HUDAssets/Audio/FlashbackSound.FlashbackSound" 1.0 1.0 0.0 0 0)
        (bind _returnvalue (UserInterface|CreateWidget "/Game/Blueprints/HUD/WBP_TextBubble.WBP_TextBubble_C" (Game|GetPlayerController 0)))
        (UserInterface|Viewport|AddtoViewport _returnvalue 0)
        (UserInterface|Animation|PlayAnimation _returnvalue (Variables|/Game/Blueprints/HUD/WBP_TextBubble.WBP_TextBubble_C|GetPopUp _returnvalue) 0.0 1 "Forward" 1.0 false)
        (Utilities|FlowControl|Delay 3.8)
        (UserInterface|Animation|PlayAnimation _returnvalue (Variables|/Game/Blueprints/HUD/WBP_TextBubble.WBP_TextBubble_C|GetDisappear _returnvalue) 0.0 1 "Forward" 1.0 false)
        (Utilities|FlowControl|Delay 0.25)
        (Widget|RemovefromParent _returnvalue)
        (bind _output_get (Variables|Default|SetRemnantCounter 0.0))
        (Variables|Default|SetRemnantsProgress _output_get)))))

(event EventBeginPlay
  (|CallParentFunction)
  (Utilities|Casting|CastToPlayerController (Pawn|GetController)))

(event Collision|EventActorBeginOverlap
  (params (OtherActor :type Actor%20Object%20Reference))
  (|CallParentFunction 0)
  (bind _asbp_collectible (Utilities|Casting|CastToBP_Collectible OtherActor))
  (Actor|DestroyActor _asbp_collectible)
  (bind _result (Math|Float|IncrementFloat (Variables|Default|GetRemnantCounter))
    (:%20%20
      (Variables|Default|SetRemnantsProgress (/ _result (Variables|Default|GetMaxRemnants)))
      (CallFunction|UnlockMemory))))

(event EventTick
  (params (DeltaSeconds :type Float%20%28single-precision%29))
  (|CallParentFunction DeltaSeconds) ; This node is disabled and will not be called.\nDrag off pins to build functionality.
)

(event Input|KeyboardEvents|Escape
  (params (Key :type Key%20Structure :default "None"))
  (bind _returnvalue (Game|GetPlayerController 0))
  (:Released
    (Game|SetGamePaused true)
    (bind _returnvalue_2 (UserInterface|CreateWidget "/Game/Blueprints/HUD/WBP_Pause.WBP_Pause_C"))
    (UserInterface|Viewport|AddtoViewport _returnvalue_2 0)
    (Input|SetInputModeUIOnly _returnvalue 0 "DoNotLock" false)
    (Variables|/Script/Engine.PlayerController|SetbShowMouseCursor _returnvalue true)))

(fn ConstructionScript
  (|CallParentFunction))