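; Guardian player character that collects Remnant pickups toward unlocking Memories and opens a pause menu on Escape.
; Pickup overlaps run collect, unlock and delayed-reset calls; the collection logic destroys pickups and advances normalized progress.
; Full progress increments Memory, shows an animated text bubble, then clears progress.
; A Win event shows a win widget at three Memories and returns to the main menu, but its visible call never runs.
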(event Custom|Win
  ;[0.15 0.15 0.15 0.5] Win state
  (if (>= (Variables|Default|GetMemory) 3)
    (bind _returnvalue (UserInterface|CreateWidget "/Game/Blueprints/HUD/WBP_Win.WBP_Win_C" (Variables|Default|GetGuardianController)))
    (UserInterface|Viewport|AddtoViewport _returnvalue 0)
    (Utilities|FlowControl|Delay 5.0)
    (Game|OpenLevel(byObjectReference) "/Game/Levels/MainMenuLevel.MainMenuLevel")))

(event Custom|MemoryUnlock1
  ;[0.15 0.15 0.15 0.5] Memory unlock conditions
  (if (>= (Variables|Default|GetRemnants%20Progress) 1.0)
    (bind _result (Math|Integer|IncrementInt (Variables|Default|GetMemory))
      (:%20%20
        (bind _output_get (Variables|Default|SetMemory _result))
        (Development|PrintString (Utilities|String|ToString(Integer) _output_get))
        (bind _returnvalue (UserInterface|CreateWidget "/Game/Blueprints/HUD/WBP_TextBubble.WBP_TextBubble_C" (Variables|Default|GetGuardianController)))
        (UserInterface|Viewport|AddtoViewport _returnvalue 0)
        (UserInterface|Animation|PlayAnimation _returnvalue (Variables|/Game/Blueprints/HUD/WBP_TextBubble.WBP_TextBubble_C|GetPopUp _returnvalue) 0.0 1 "Forward" 1.0 false)
        (Utilities|FlowControl|Delay 3.8)
        (UserInterface|Animation|PlayAnimation _returnvalue (Variables|/Game/Blueprints/HUD/WBP_TextBubble.WBP_TextBubble_C|GetDisappear _returnvalue) 0.0 1 "Forward" 1.0 false)
        (Utilities|FlowControl|Delay 0.25)
        (Widget|RemovefromParent _returnvalue)
        (bind _output_get_2 (Variables|Default|SetRemnants%20Counter 0.0))
        (Variables|Default|SetRemnants%20Progress _output_get_2)))))

(event EventBeginPlay
  ;[0.15 0.15 0.15 0.5] get HUD to work
  (|CallParentFunction)
  (bind _asguardian_controller (Utilities|Casting|CastToGuardianController (Game|GetPlayerController 0)))
  (Utilities|Casting|CastToBP_HUD (HUD|GetHUD _asguardian_controller)))

(event Collision|EventActorBeginOverlap
  (params (OtherActor :type Actor%20Object%20Reference))
  ;[0.15 0.15 0.15 0.5] Collecting Remnants
  (|CallParentFunction 0)
  (bind _aspickup (Utilities|Casting|CastToPickup OtherActor))
  (Class|GuardianCharacter|RemnantCollect _aspickup)
  (Class|GuardianCharacter|MemoryUnlock)
  (Utilities|FlowControl|Delay 3.8)
  (Class|GuardianCharacter|ResetRemnantProgress))

(event EventTick
  (params (DeltaSeconds :type Float%20%28single-precision%29)))

(event Input|KeyboardEvents|Escape
  (params (Key :type Key%20Structure :default "None"))
  (bind _returnvalue (Game|GetPlayerController 0))
  ;[0.15 0.15 0.15 0.5] Pause
  (:Released
    (Game|SetGamePaused true)
    (bind _returnvalue_2 (UserInterface|CreateWidget "/Game/Blueprints/HUD/WBP_Pause.WBP_Pause_C" (Variables|Default|GetGuardianController)))
    (UserInterface|Viewport|AddtoViewport _returnvalue_2 0)
    (Input|SetInputModeUIOnly _returnvalue 0 "DoNotLock" false)
    (Variables|/Script/Engine.PlayerController|SetbShowMouseCursor _returnvalue true)))

(fn ConstructionScript)

(fn NewFunction
  (params (Object :type Object%20Object%20Reference))
  (if (< (Variables|Default|GetRemnants%20Progress) 1.0)
    (bind _aspickup (Utilities|Casting|CastToPickup Object))
    (if (Variables|/Script/CrescentRemnants.Pickup|GetbIsPickup _aspickup)
      (Actor|DestroyActor _aspickup)
      (bind _result (Math|Float|IncrementFloat (Variables|Default|GetRemnants%20Counter))
        (:%20%20
          (bind _output_get (Variables|Default|SetRemnants%20Progress (/ _result (Variables|Default|GetMax%20Remnants))))
          (Development|PrintString (Utilities|String|ToString(Float) _output_get)))))))