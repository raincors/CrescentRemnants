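; Enemy AI actor that chases the Guardian player character and snaps back to its spawn transform when the two overlap.
; PlayerSensing sets PlayerSeen and starts an AIMoveTo toward the Guardian, while Tick caches the player's position.
; A self-recursing Patrol event moves back and forth along X until the player is seen, but nothing in this graph calls it.
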(event OnSeePawn(PlayerSensing)
  (params (Pawn :type Pawn%20Object%20Reference))
  (bind _asbp_guardian_character (Utilities|Casting|CastToBP_GuardianCharacter Pawn))
  (Variables|Default|SetPlayerSeen true)
  (bind _output_get (Variables|Default|SetPlayer _asbp_guardian_character))
  (AI|AIMoveTo self (Variables|Default|GetCurrentPlayerPos) _output_get 1.0 true))

(event Custom|GuardianPosition
  (Variables|Default|SetCurrentPlayerPos (Transformation|GetActorLocation (Game|GetPlayerCharacter 0))))

(event Custom|Patrol
  (bind _returnvalue (Transformation|GetActorLocation))
  (while (!= (Variables|Default|GetPlayerSeen) true)
    (AI|AIMoveTo 0 (Math|Vector|MakeVector (+ (Variables|Default|GetPatrolDistance) (.x _returnvalue)) (.y _returnvalue) (.z _returnvalue)) 0 5.0 false
      (:then
        (AI|AIMoveTo 0 (Math|Vector|MakeVector (- (.x (Transformation|GetActorLocation)) (Variables|Default|GetPatrolDistance)) (.y _returnvalue) (.z _returnvalue)) 0 5.0 false
          (:then
            (CallFunction|Patrol)))))))

(event EventBeginPlay
  (Variables|Default|SetOriginalLocation (Transformation|GetActorLocation))
  (Variables|Default|SetOriginalRotation (Transformation|GetActorRotation))
  (Variables|Default|SetPlayerSeen false))

(event Collision|EventActorBeginOverlap
  (params (OtherActor :type Actor%20Object%20Reference))
  (Utilities|Casting|CastToBP_GuardianCharacter OtherActor)
  (Transformation|SetActorRotation (Variables|Default|GetOriginalRotation))
  (Transformation|SetActorLocation (Variables|Default|GetOriginalLocation) false false))

(event EventTick
  (params (DeltaSeconds :type Float%20%28single-precision%29))
  (CallFunction|GuardianPosition))

(fn ConstructionScript)